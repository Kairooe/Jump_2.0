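; BP_JumpPad_Sideway is a jump pad that launches the player upward and reverses their RightLeft direction value.
; On BeginPlay it caches the first BP_ThirdPersonCharacter in the level.
; Any actor overlap prints a "Wall Hit" debug string and negates that cached character's RightLeft, without checking the overlapping actor.
; Box overlaps cast to the character and launch it with boosted JumpZVelocity, overriding vertical velocity.
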(event `CharRef`
  (bind _outactors (`GameplayStatics.GetAllActorsOfClass` "/Game/ThirdPerson/Blueprints/BP_ThirdPersonCharacter.BP_ThirdPersonCharacter_C"))
  (set `self.3rdPlayer_right Left` (`|GetArrayItem` _outactors)))

(event `self.ReceiveBeginPlay`
  (`self.CharRef`))

(event `self.ReceiveActorBeginOverlap`
  (params (OtherActor :type "Actor Object Reference"))
  (`KismetSystemLibrary.PrintString` "Wall Hit")
  (set `/Game/ThirdPerson/Blueprints/BP_ThirdPersonCharacter.Right/Left` (* -1.0 (`/Game/ThirdPerson/Blueprints/BP_ThirdPersonCharacter.Right/Left` (`self.3rdPlayer_right Left`))) (`self.3rdPlayer_right Left`)))

(event `self.Box.OnComponentBeginOverlap`
  (params (OverlappedComponent :type "PrimitiveComponent Object Reference") (OtherActor :type "Actor Object Reference") (OtherComp :type "PrimitiveComponent Object Reference") (OtherBodyIndex :type Integer) (bFromSweep :type Boolean) (SweepResult :type "HitResult Structure (by ref)"))
  (bind _asbp_third_person_character (cast `/Game/ThirdPerson/Blueprints/BP_ThirdPersonCharacter` OtherActor))
  (`Character.LaunchCharacter` _asbp_third_person_character (`KismetMathLibrary.MakeVector` 0.0 0.0 (* (`CharacterMovementComponent.JumpZVelocity` (`Character.CharacterMovement` _asbp_third_person_character)) 1.5)) false true))

(fn `UserConstructionScript`)