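; BP_WallNoTop is a wall prefab that reverses the player character's left-right direction on contact.
; On BeginPlay it finds the first BP_ThirdPersonCharacter in the level and caches it.
; Any actor overlap prints a debug "Wall Hit" and negates that character's RightLeft value, without checking which actor overlapped.
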(event `CharRef`
  (bind _outactors (`GameplayStatics.GetAllActorsOfClass` "/Game/ThirdPerson/Blueprints/BP_ThirdPersonCharacter.BP_ThirdPersonCharacter_C"))
  (set `self.3rdPlayer_right Left` (`|GetArrayItem` _outactors)))

(event `self.ReceiveBeginPlay`
  (`self.CharRef`))

(event `self.ReceiveActorBeginOverlap`
  (params (OtherActor :type "Actor Object Reference"))
  (`KismetSystemLibrary.PrintString` "Wall Hit")
  (set `/Game/ThirdPerson/Blueprints/BP_ThirdPersonCharacter.Right/Left` (* -1.0 (`/Game/ThirdPerson/Blueprints/BP_ThirdPersonCharacter.Right/Left` (`self.3rdPlayer_right Left`))) (`self.3rdPlayer_right Left`)))

(fn `UserConstructionScript`)