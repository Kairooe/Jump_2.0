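; Warp pipe trigger that teleports any actor entering its Box to an Arrow destination and reverses the third-person character's RightLeft direction value.
; The construction script places the Arrow from the TeleportLocation transform.
; On BeginPlay it caches the first BP_ThirdPersonCharacter, whose RightLeft is negated on every overlap, whichever actor enters.
; When the player is teleported, control rotation is matched to the new facing and velocity is zeroed.
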(event `CharRef`
  (bind _outactors (`GameplayStatics.GetAllActorsOfClass` "/Game/ThirdPerson/Blueprints/BP_ThirdPersonCharacter.BP_ThirdPersonCharacter_C"))
  (set `self.3rdPlayer_right Left` (`|GetArrayItem` _outactors)))

(event `self.ReceiveBeginPlay`
  (`self.CharRef`))

(event `self.Box.OnComponentBeginOverlap`
  (params (OverlappedComponent :type "PrimitiveComponent Object Reference") (OtherActor :type "Actor Object Reference") (OtherComp :type "PrimitiveComponent Object Reference") (OtherBodyIndex :type Integer) (bFromSweep :type Boolean) (SweepResult :type "HitResult Structure (by ref)"))
  (bind _returnvalue (`GameplayStatics.GetPlayerCharacter` 0))
  (bind (_returnvalue_location _returnvalue_rotation) (`KismetMathLibrary.BreakTransform` (`SceneComponent.K2_GetComponentToWorld` (`self.Arrow`))))
  (`|ExecutionSequence`
    (:`then_0`
      (`KismetSystemLibrary.PrintString` "Wall Hit")
      (set `/Game/ThirdPerson/Blueprints/BP_ThirdPersonCharacter.Right/Left` (* -1.0 (`/Game/ThirdPerson/Blueprints/BP_ThirdPersonCharacter.Right/Left` (`self.3rdPlayer_right Left`))) (`self.3rdPlayer_right Left`)))
    (:`then_1`
      (`SceneComponent.K2_SetWorldTransform` (`Actor.RootComponent` OtherActor) (`KismetMathLibrary.MakeTransform` _returnvalue_location _returnvalue_rotation) false false)
      (if (== OtherActor _returnvalue)
        (`Controller.SetControlRotation` (`GameplayStatics.GetPlayerController` 0) (`self.K2_GetActorRotation` _returnvalue))
        (set `MovementComponent.Velocity` (0.0 0.0 0.0) (`Character.CharacterMovement` _returnvalue))))))

(fn `UserConstructionScript`
  (`SceneComponent.K2_SetRelativeTransform` (`self.Arrow`) (`self.Teleport Location`) false false))